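; BP_HUD_CharacterSelect is a HUD Blueprint that displays the selected-unit window for unit selection.
; On BeginPlay it creates the WB_HUD_CharacterSelect widget, keeps a reference and adds it to the viewport.
; ShowSelectedUnitWindow clears the window, then refreshes the nested WBUnitSelection widget with the selected actor.
; RemoveSelectedUnitWindow clears it by calling the same RefreshWidget with no actor.
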(event `self.ReceiveBeginPlay`
  (bind _returnvalue (`|CreateWidget` "/Game/UnitSelection/HUD/WB_HUD_CharacterSelect.WB_HUD_CharacterSelect_C"))
  (bind _output_get (set `self.AsWBHUD` _returnvalue))
  (`UserWidget.AddToViewport` _output_get 0))

(fn `RemoveSelectedUnitWindow`
  (bind _aswbhud (`self.AsWBHUD`)
    (:`then`
      (`/Game/UnitSelection/Character/UI/WB_UnitSelection.RefreshWidget` (`/Game/UnitSelection/HUD/WB_HUD_CharacterSelect.WB_UnitSelection` _aswbhud) null))
    (:`else`)))

(fn `ShowSelectedUnitWindow`
  (params (SelectedActor :type "Actor Object Reference"))
  (`self.RemoveSelectedUnitWindow`)
  (bind _aswbhud (`self.AsWBHUD`)
    (:`then`
      (`/Game/UnitSelection/Character/UI/WB_UnitSelection.RefreshWidget` (`/Game/UnitSelection/HUD/WB_HUD_CharacterSelect.WB_UnitSelection` _aswbhud) SelectedActor))
    (:`else`)))

(fn `UserConstructionScript`)