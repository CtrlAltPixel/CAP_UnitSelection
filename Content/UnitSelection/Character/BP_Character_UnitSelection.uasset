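; Selectable unit character with a hover outline, selection marker and screen-space nameplate.
; Construction makes the capsule block a custom trace channel and sizes the hidden Selection marker to the capsule's diameter.
; BeginPlay requires the unit-selection player controller, tints the marker cyan, stops the mesh receiving decals and creates the nameplate widget showing the unit's name.
; Cursor-over events apply and clear a cyan dynamic outline through the mesh's overlay material.
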(event `self.ReceiveBeginPlay`
  (bind _selection (`self.Selection`))
  (bind _asbp_pc_unit_selection (cast `/Game/UnitSelection/Player/BP_PC_UnitSelection` (`GameplayStatics.GetPlayerController` 0)))
  (set `self.As BP Top Down Controller` _asbp_pc_unit_selection)
  (bind _returnvalue (`PrimitiveComponent.CreateDynamicMaterialInstance` _selection 0 (`PrimitiveComponent.GetMaterial` _selection 0) "None"))
  (`MaterialInstanceDynamic.SetVectorParameterValue` _returnvalue "Colour" (struct :`G` 1.0 :`B` 1.0 :`A` 1.0))
  (`self.InitUnit`))

(event `InitUnit`
  (`PrimitiveComponent.SetReceivesDecals` (`self.Mesh`) false)
  (`self.CreateUnitHUD`))

(event `CreateUnitHUD`
  (bind _wb_unithud (`self.WB_UnitHUD`))
  (bind _returnvalue (`|CreateWidget` "/Game/UnitSelection/Character/UI/WB_UnitNameplate.WB_UnitNameplate_C" null self))
  (bind _output_get (set `self.As WB_UnitHUD` _returnvalue))
  (set `/Game/UnitSelection/Character/UI/WB_UnitNameplate.As OwningUnit` self _output_get)
  (`TextBlock.SetText` (`/Game/UnitSelection/Character/UI/WB_UnitNameplate.TextBlock_Username` _output_get) (`self.Name`))
  (`WidgetComponent.SetWidget` _wb_unithud _output_get)
  (`WidgetComponent.SetWidgetSpace` _wb_unithud "Screen")
  (`WidgetComponent.SetDrawAtDesiredSize` _wb_unithud true))

(event `self.ReceiveActorBeginCursorOver`
  (bind _returnvalue (`KismetMaterialLibrary.CreateDynamicMaterialInstance` "/Game/UnitSelection/Character/Materials/MAT_OutlineOverlay.MAT_OutlineOverlay"))
  (bind _output_get (set `self.OverlayMaterial` _returnvalue))
  (`MeshComponent.SetOverlayMaterial` (`self.Mesh`) _output_get)
  (`MaterialInstanceDynamic.SetVectorParameterValue` (`self.OverlayMaterial`) "Colour" (struct :`G` 1.0 :`B` 1.0 :`A` 1.0)))

(event `self.ReceiveActorEndCursorOver`
  (`MeshComponent.SetOverlayMaterial` (`self.Mesh`) null))

(fn `UserConstructionScript`
  (bind _selection (`self.Selection`))
  (`PrimitiveComponent.SetCollisionResponseToChannel` (`self.CapsuleComponent`) "ECC_GameTraceChannel1" "ECR_Block")
  (`SceneComponent.SetVisibility` _selection false false)
  (`SceneComponent.SetWorldScale3D` _selection (`KismetMathLibrary.Conv_DoubleToVector` (/ (* (`CapsuleComponent.CapsuleRadius` (`self.CapsuleComponent`)) 2.0) 100.0))))