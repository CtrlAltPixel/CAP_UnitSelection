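; Selectable unit character that shows hover and interaction feedback and carries a screen-space nameplate with its name.
; BeginPlay creates dynamic outline and decal materials, sets the unit-selection AI controller class and builds the nameplate widget.
; Cursor hover toggles a cyan mesh outline overlay, while interact begin/end events toggle a ground decal scaled from the capsule radius.
; The capsule blocks a custom trace channel.
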(event `self.ReceiveBeginPlay`
  (`self.InitMatOutlineOverlay`)
  (`self.InitMatDecalInteract`)
  (`self.InitCharacter`)
  (`self.CreateUnitHUD`))

(event `CreateUnitHUD`
  (bind _wb_unithud (`self.WB_UnitHUD`))
  (bind _returnvalue (`|CreateWidget` "/Game/UnitSelection/Character/UI/WB_UnitNameplate.WB_UnitNameplate_C" null self))
  (bind _output_get (set `self.As WB_UnitHUD` _returnvalue))
  (set `/Game/UnitSelection/Character/UI/WB_UnitNameplate.As OwningUnit` self _output_get)
  (`TextBlock.SetText` (`/Game/UnitSelection/Character/UI/WB_UnitNameplate.TextBlock_Username` _output_get) (`self.Name`))
  (`WidgetComponent.SetWidget` _wb_unithud _output_get)
  (`WidgetComponent.SetWidgetSpace` _wb_unithud "Screen")
  (`WidgetComponent.SetDrawAtDesiredSize` _wb_unithud true))

(event `BeginActorInteract`
  (`SceneComponent.SetVisibility` (`self.Decal_Interact`) true false))

(event `EndActorInteract`
  (`SceneComponent.SetVisibility` (`self.Decal_Interact`) false false))

(event `self.ReceiveActorBeginCursorOver`
  (`MeshComponent.SetOverlayMaterial` (`self.Mesh`) (`self.MATOverlayOutline`))
  (`MaterialInstanceDynamic.SetVectorParameterValue` (`self.MATOverlayOutline`) "Colour" (struct :`G` 1.0 :`B` 1.0 :`A` 1.0)))

(event `self.ReceiveActorEndCursorOver`
  (`MeshComponent.SetOverlayMaterial` (`self.Mesh`) null))

(fn `InitCharacter`
  (`PrimitiveComponent.SetCollisionResponseToChannel` (`self.CapsuleComponent`) "ECC_GameTraceChannel1" "ECR_Block")
  (`PrimitiveComponent.SetReceivesDecals` (`self.Mesh`) false)
  (`SceneComponent.SetVisibility` (`self.Decal_Interact`) false false)
  (set `self.AIControllerClass` "/Game/UnitSelection/Character/AI/BP_AIController_UnitSelection.BP_AIController_UnitSelection_C"))

(fn `InitMatDecalInteract`
  (bind _returnvalue (`KismetMaterialLibrary.CreateDynamicMaterialInstance` "/Game/UnitSelection/Character/Materials/MAT_DecalSelect.MAT_DecalSelect"))
  (bind _output_get (set `self.MATDecalInteract` _returnvalue))
  (`MaterialInstanceDynamic.SetVectorParameterValue` _output_get "Colour" (struct :`G` 1.0 :`B` 1.0 :`A` 1.0)))

(fn `InitMatOutlineOverlay`
  (bind _returnvalue (`KismetMaterialLibrary.CreateDynamicMaterialInstance` "/Game/UnitSelection/Character/Materials/MAT_OutlineOverlay.MAT_OutlineOverlay"))
  (bind _output_get (set `self.MATOverlayOutline` _returnvalue))
  (`MaterialInstanceDynamic.SetVectorParameterValue` :`self` _output_get))

(fn `UserConstructionScript`
  (bind _decal_interact (`self.Decal_Interact`))
  (`PrimitiveComponent.SetCollisionResponseToChannel` (`self.CapsuleComponent`) "ECC_GameTraceChannel1" "ECR_Block")
  (`SceneComponent.SetVisibility` _decal_interact false false)
  (`SceneComponent.SetWorldScale3D` _decal_interact (`KismetMathLibrary.Conv_DoubleToVector` (/ (* (`CapsuleComponent.CapsuleRadius` (`self.CapsuleComponent`)) 2.0) 100.0))))