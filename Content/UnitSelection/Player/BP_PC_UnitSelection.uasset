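; Player controller for a unit selection game that picks units with the mouse and shows the selected one on the HUD.
; On begin play it adds the default input mapping, caches the HUD and enables cursor, click and hover events.
; The primary action traces under the cursor, stores a hit unit character and shows its window, otherwise removing the window.
; Helpers for click-to-move, follow and touch location are defined but not called here.
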(event `self.ReceiveBeginPlay`
  (bind _returnvalue (subsystem `EnhancedInputLocalPlayerSubsystem`))
  ;[0.05098 0.05098 0.05098] Add Mapping Context
  (`/Engine/EditorBlueprintResources/StandardMacros.IsValid` _returnvalue
    (:`Is Valid`
      (`EnhancedInputSubsystemInterface.AddMappingContext` _returnvalue "/Game/UnitSelection/Input/IMC_Default.IMC_Default" 0 (struct))
      (if (`self.IsLocalPlayerController`)
        (bind _asbp_hud_unit_selection (cast `/Game/UnitSelection/HUD/BP_HUD_UnitSelection` (`self.GetHUD`)))
        (set `self.As BP HUD Unit Selection` _asbp_hud_unit_selection)
        (`WidgetBlueprintLibrary.SetInputMode_GameAndUIEx` self null "DoNotLock" false)
        (set `self.CurrentClickTraceChannel` "ECC_GameTraceChannel1")
        (set `self.bShowMouseCursor` true)
        (set `self.bEnableClickEvents` true)
        (set `self.bEnableMouseOverEvents` true)))))

(event `EnhancedInput|/Game/UnitSelection/Input/Actions/IA_PrimaryAction`
  (params (ActionValue :type Boolean) (ElapsedSeconds :type "Float (double-precision)") (TriggeredSeconds :type "Float (double-precision)") (InputAction :type "InputAction Object Reference" :default "/Game/UnitSelection/Input/Actions/IA_PrimaryAction.IA_PrimaryAction"))
  (bind (_hit _hitactor) (`self.GetActorUnderCursor`))
  (:`Triggered`
    (if (`GameplayStatics.ObjectIsA` _hitactor "/Game/UnitSelection/Character/BP_Character_UnitSelection.BP_Character_UnitSelection_C")
      (`self.SetSelectedUnit` _hitactor)
      (else
        (bind _as_bp_hud_unit_selection (`self.As BP HUD Unit Selection`)
          (:`then`
            (`/Game/UnitSelection/HUD/BP_HUD_UnitSelection.RemoveSelectedUnitWindow` _as_bp_hud_unit_selection))
          (:`else`))))))

(fn `Follow`
  (params (Location :type "Vector Structure"))
  (bind _returnvalue (`self.K2_GetPawn`))
  (`Pawn.AddMovementInput` _returnvalue (`KismetMathLibrary.GetDirectionUnitVector` (`self.K2_GetActorLocation` _returnvalue) Location) 1.0 false))

(fn `GetActorUnderCursor`
  (returns (Hit :type Boolean) (HitActor :type "Actor Object Reference"))
  (bind (_bblockinghit _binitialoverlap _time _distance _location _impactpoint _normal _impactnormal _physmat _hitactor) (`GameplayStatics.BreakHitResult` (`self.GetHitResultUnderCursorByChannel` "TraceTypeQuery3")))
  (return _bblockinghit _hitactor))

(fn `GetLocationUnderCursor`
  (returns (Hit :type Boolean) (Location :type "Vector Structure"))
  (bind (_bblockinghit _binitialoverlap _time _distance _location) (`GameplayStatics.BreakHitResult` (`self.GetHitResultUnderCursorByChannel` "TraceTypeQuery1")))
  (return _bblockinghit _location))

(fn `GetLocationUnderFinger`
  (returns (Hit :type Boolean) (Location :type "Vector Structure"))
  (bind (_bblockinghit _binitialoverlap _time _distance _location) (`GameplayStatics.BreakHitResult` (`self.GetHitResultUnderFingerByChannel` "Touch1" "TraceTypeQuery1" false)))
  (return _bblockinghit _location))

(fn `MoveTo`
  (params (Location :type "Vector Structure"))
  (`AIBlueprintHelperLibrary.SimpleMoveToLocation` self Location)
  (`NiagaraFunctionLibrary.SpawnSystemAtLocation` (`self.FXCursor`) Location))

(fn `SetSelectedUnit`
  (params (SelectedActor :type "Actor Object Reference"))
  (bind _output_get (set `self.SelectedUnit` SelectedActor))
  (bind _as_bp_hud_unit_selection (`self.As BP HUD Unit Selection`)
    (:`then`
      (`/Game/UnitSelection/HUD/BP_HUD_UnitSelection.ShowSelectedUnitWindow` _as_bp_hud_unit_selection _output_get))
    (:`else`)))

(fn `UserConstructionScript`)