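; Player controller for the character selection scene, handling camera control and clicking on units with a visible mouse cursor.
; On BeginPlay it adds Enhanced Input contexts for camera and interaction and caches the HUD and camera pawn, which receives move and drag input.
; Pressing interact clears the selection window and traces under the cursor: a hit character opens its HUD window, while empty space temporarily enables the drag mapping context.
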(event `self.ReceiveBeginPlay`
  (bind _returnvalue (subsystem `EnhancedInputLocalPlayerSubsystem`))
  ;[0.05098 0.05098 0.05098] Add Mapping Context
  (if (`self.IsLocalPlayerController`)
    (`/Engine/EditorBlueprintResources/StandardMacros.IsValid` _returnvalue
      (:`Is Valid`
        (`EnhancedInputSubsystemInterface.AddMappingContext` _returnvalue "/Game/UnitSelection/Input/IMC_Camera.IMC_Camera" 0 (struct))
        (`EnhancedInputSubsystemInterface.AddMappingContext` _returnvalue "/Game/UnitSelection/Input/IMC_Interact.IMC_Interact" 0 (struct))
        (`self.InitCasts`)
        (`WidgetBlueprintLibrary.SetInputMode_GameAndUIEx` self null "DoNotLock" false)
        (set `self.CurrentClickTraceChannel` "ECC_GameTraceChannel1")
        (set `self.bShowMouseCursor` true)
        (set `self.bEnableClickEvents` true)
        (set `self.bEnableMouseOverEvents` true)))))

(event `EnhancedInput|/Game/UnitSelection/Input/Actions/IA_CameraMove`
  (params (ActionValue :type "Vector2D Structure") (ElapsedSeconds :type "Float (double-precision)") (TriggeredSeconds :type "Float (double-precision)") (InputAction :type "InputAction Object Reference" :default "/Game/UnitSelection/Input/Actions/IA_CameraMove.IA_CameraMove"))
  (:`Triggered`
    (bind _as_bp_pawn_camera_character_select (`self.As BP Pawn Camera Character Select`)
      (:`then`
        (`/Game/UnitSelection/Camera/BP_Pawn_Camera_CharacterSelect.CameraMove` _as_bp_pawn_camera_character_select ActionValue_X ActionValue_Y))
      (:`else`))))

(event `EnhancedInput|/Game/UnitSelection/Input/Actions/IA_Drag`
  (params (ActionValue :type "Vector2D Structure") (ElapsedSeconds :type "Float (double-precision)") (TriggeredSeconds :type "Float (double-precision)") (InputAction :type "InputAction Object Reference" :default "/Game/UnitSelection/Input/Actions/IA_Drag.IA_Drag"))
  (:`Triggered`
    (bind _as_bp_pawn_camera_character_select (`self.As BP Pawn Camera Character Select`)
      (:`then`
        (`/Game/UnitSelection/Camera/BP_Pawn_Camera_CharacterSelect.CameraDrag` _as_bp_pawn_camera_character_select ActionValue_X ActionValue_Y))
      (:`else`))))

(event `EnhancedInput|/Game/UnitSelection/Input/Actions/IA_Interact`
  (params (ActionValue :type Boolean) (ElapsedSeconds :type "Float (double-precision)") (TriggeredSeconds :type "Float (double-precision)") (InputAction :type "InputAction Object Reference" :default "/Game/UnitSelection/Input/Actions/IA_Interact.IA_Interact"))
  (bind (_hit _hitactor) (`self.GetActorUnderCursorByChannel` "TraceTypeQuery3"))
  (:`Triggered`
    (if (`GameplayStatics.ObjectIsA` (`self.InteractActor`) "/Game/UnitSelection/Character/BP_Character_CharacterSelection.BP_Character_CharacterSelection_C")
      (`self.SetSelectedUnit` (`self.InteractActor`))))
  (:`Started`
    (bind _as_bp_hud_unit_selection (`self.As BP HUD Unit Selection`)
      (:`then`
        (`/Game/UnitSelection/HUD/BP_HUD_CharacterSelect.RemoveSelectedUnitWindow` _as_bp_hud_unit_selection))
      (:`else`
        _))
    (if _hit
      (set `self.InteractActor` _hitactor)
      (else
        (`EnhancedInputSubsystemInterface.AddMappingContext` (subsystem `EnhancedInputLocalPlayerSubsystem`) "/Game/UnitSelection/Input/IMC_Drag.IMC_Drag" 0 (struct)))))
  (:`Canceled`
    (`EnhancedInputSubsystemInterface.RemoveMappingContext` (subsystem `EnhancedInputLocalPlayerSubsystem`) "/Game/UnitSelection/Input/IMC_Drag.IMC_Drag" (struct))))

(fn `GetActorUnderCursorByChannel`
  (params (TraceChannel :type "ETraceTypeQuery Enum" :default "TraceTypeQuery1"))
  (returns (Hit :type Boolean) (HitActor :type "Actor Object Reference"))
  (bind (_bblockinghit _binitialoverlap _time _distance _location _impactpoint _normal _impactnormal _physmat _hitactor) (`GameplayStatics.BreakHitResult` (`self.GetHitResultUnderCursorByChannel` TraceChannel)))
  (return _bblockinghit _hitactor))

(fn `InitCasts`
  (bind _asbp_hud_character_select (cast `/Game/UnitSelection/HUD/BP_HUD_CharacterSelect` (`self.GetHUD`)))
  (set `self.As BP HUD Unit Selection` _asbp_hud_character_select)
  (bind _asbp_pawn_camera_character_select (cast `/Game/UnitSelection/Camera/BP_Pawn_Camera_CharacterSelect` (`self.K2_GetPawn`)))
  (set `self.As BP Pawn Camera Character Select` _asbp_pawn_camera_character_select))

(fn `SetSelectedUnit`
  (params (SelectedActor :type "Actor Object Reference"))
  (bind _asbp_character_character_selection (cast `/Game/UnitSelection/Character/BP_Character_CharacterSelection` SelectedActor))
  (bind _output_get (set `self.As BP Character Character Selection` _asbp_character_character_selection))
  (bind _as_bp_hud_unit_selection (`self.As BP HUD Unit Selection`)
    (:`then`
      (`/Game/UnitSelection/HUD/BP_HUD_CharacterSelect.ShowSelectedUnitWindow` _as_bp_hud_unit_selection _output_get))
    (:`else`)))

(fn `UserConstructionScript`)